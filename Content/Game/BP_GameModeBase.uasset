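; Base game mode Blueprint that handles level transitions: advancing to the next level, opening a level by ID, and restarting the current one.
; Each event asks the LF default content object to resolve the target level, using either the game mode as context or the given ID.
; The resolved level is opened by object reference as an absolute travel with no options.
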(event Custom|OpenNextLevel
  (bind _returnvalue (Class|LFDefaultContent|GetNextLevel (Class|LFLibrary|GetLFDefaultContent) self))
  (Game|OpenLevel(byObjectReference) _returnvalue))

(event Custom|RestartLevel
  (bind _returnvalue (Class|LFDefaultContent|GetCurrentLevel (Class|LFLibrary|GetLFDefaultContent) self))
  (Game|OpenLevel(byObjectReference) _returnvalue))

(event Custom|OpenLevelByID
  (params (NewParam :type Integer))
  (bind _returnvalue (Class|LFDefaultContent|GetLevel (Class|LFLibrary|GetLFDefaultContent) NewParam))
  (Game|OpenLevel(byObjectReference) _returnvalue))

(fn ConstructionScript)