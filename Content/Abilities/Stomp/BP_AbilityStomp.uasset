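; Character stomp ability that slams down to break objects with a stomp-breakable component.
; From the ground it triggers a jump first, then freezes movement at the recorded height and restores falling with extreme gravity after a timed pause.
; Capsule hits while stomp is unavailable pass the drop height to breakables.
; Landing restores gravity and starts the cooldown; the destroy-below function is an empty stub.
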(event Custom|TryToReenable
  (params (PrevMovementMode :type EMovementMode%20Enum :default "MOVE_None") (NewMovementMode :type EMovementMode%20Enum :default "MOVE_None"))
  ;[1 1 1] We can't stamp again until we land
  (if (and (Utilities|Enum|Equal(Enum) PrevMovementMode "MOVE_Falling") (Utilities|Enum|Equal(Enum) NewMovementMode "MOVE_Walking"))
    (CallFunction|OnLanded)))

(event Custom|TryToBreakOtherActor
  (params (HitComponent :type Primitive%20Component%20Object%20Reference) (OtherActor :type Actor%20Object%20Reference) (OtherComp :type Primitive%20Component%20Object%20Reference) (NormalImpulse :type Vector) (Hit :type Hit%20Result%20Structure%20%28by%20ref%29))
  (bind _returnvalue (Actor|GetComponentbyClass OtherActor "/Game/Components/BP_StompBreakableComponent.BP_StompBreakableComponent_C"))
  (if (not (Variables|Default|GetbIsAbleToStomp))
    (Utilities|IsValid _returnvalue
      (:Is%20Valid
        (Default|Stomp _returnvalue (- (Variables|Default|GetCachedHighestStompPoint) (.Z (Math|Vector|BreakVector (Transformation|GetActorLocation (Variables|Default|GetOwnerCharacter))))))))))

(event Custom|ResetAbility
  (Variables|Default|SetbIsAbleToStomp true))

(event EventBeginAbility
  (params (Character :type LF%20Character%20Object%20Reference) (AbilityComponent :type LF%20Ability%20Component%20Object%20Reference))
  (|CallParentFunction Character AbilityComponent)
  (bind _asbp_character (Utilities|Casting|CastToBP_Character Character))
  (EventDispatchers|BindEventtoOnMovementChanged _asbp_character (delegate Custom|TryToReenable))
  (Collision|BindEventtoOnComponentHit (Variables|/Script/Engine.Character|GetCapsuleComponent _asbp_character) (delegate Custom|TryToBreakOtherActor)))

(event EventActivateAbility
  (|CallParentFunction)
  (Variables|Default|SetbIsAbleToStomp false)
  (if (AI|Components|NavMovement|IsFalling (Variables|/Script/Engine.Character|GetCharacterMovement (Variables|Default|GetOwnerCharacter)))
    (CallFunction|StartStompAnimation)
    (else
      (CallFunction|SmallJump))))

(event EventDeactivateAbility
  (|CallParentFunction)
  (Variables|/Script/Engine.CharacterMovementComponent|SetGravityScale (Variables|/Script/Engine.Character|GetCharacterMovement (Variables|Default|GetOwnerCharacter)) (Variables|Default|GetCachedGravityScale))
  (Utilities|Time|SetTimerbyEvent (delegate Custom|ResetAbility) (Variables|Configuration|GetCooldown)))

(fn CanUseAbility
  (bind _returnvalue (|CallParentFunction))
  (return (and _returnvalue (Variables|Default|GetbIsAbleToStomp))))

(fn StartStompAnimation
  (bind _ownercharacter (Variables|Default|GetOwnerCharacter))
  (Pawn|Components|CharacterMovement|DisableMovement (Variables|/Script/Engine.Character|GetCharacterMovement _ownercharacter))
  (Variables|Default|SetCachedHighestStompPoint (.Z (Math|Vector|BreakVector (Transformation|GetActorLocation _ownercharacter))))
  (Utilities|Time|SetTimerbyFunctionName 0 "StompFall" (Variables|Configuration|GetTimeStompAnimation)))

(fn SmallJump
  (Utilities|Time|SetTimerbyFunctionName 0 "StartStompAnimation" (Variables|Configuration|GetTimeJumpAnimation))
  (Class|LFAbilityComponent|ActivateAbilitybyType (Variables|Default|GetOwnerAbilityComponent) "Jump")
  ;[1 1 1] TODO Delete this once an ability is created?
  (Character|Jump (Variables|Default|GetOwnerCharacter)))

(fn StompFall
  (bind _ownercharacter (Variables|Default|GetOwnerCharacter))
  (bind _charactermovement (Variables|/Script/Engine.Character|GetCharacterMovement _ownercharacter))
  (Pawn|Components|CharacterMovement|SetMovementMode _charactermovement "MOVE_Falling" 0)
  (Variables|Default|SetCachedGravityScale (Variables|/Script/Engine.CharacterMovementComponent|GetGravityScale _charactermovement))
  (Variables|/Script/Engine.CharacterMovementComponent|SetGravityScale _charactermovement 1e+05))

(fn OnLanded
  (if (Variables|Default|GetbIsAbleToStomp)
    (Variables|Default|SetbIsAbleToStomp true)
    (else
      (CallFunction|TrytoDestroyObjectBelow)
      (Class|LFAbility|DeactivateAbility))))

(fn TrytoDestroyObjectBelow)