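; Jetpack ability that lifts the owning character for a limited time, with jetpack FX toggled on the character.
; Activation zeroes velocity, then each running update relaunches the character upward at a speed derived from max height over max time.
; Timeout deactivates it through the ability component, cancelling vertical velocity and leaving it stilled until landing from a fall restores readiness.
; Use requires the ready state and is blocked during Stomp.
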(event Custom|MovementModeChangedDelegate_Event_0
  (params (Character :type Character%20Object%20Reference) (PrevMovementMode :type EMovementMode%20Enum :default "MOVE_None") (PreviousCustomMode :type Byte))
  (if (|ComesfromFall PrevMovementMode Character)
    (Variables|Default|SetJetpackState "NewEnumerator0")
    (Variables|Default|SetCurrentJetpackTime 0.0)))

(event EventBeginAbility
  (params (Character :type LF%20Character%20Object%20Reference) (AbilityComponent :type LF%20Ability%20Component%20Object%20Reference))
  (|CallParentFunction Character AbilityComponent)
  (Character|AssignMovementModeChangedDelegate Character (delegate Custom|MovementModeChangedDelegate_Event_0)))

(event EventActivateAbility
  (bind _ownercharacter (Variables|Default|GetOwnerCharacter))
  (bind _charactermovement (Variables|/Script/Engine.Character|GetCharacterMovement _ownercharacter))
  (|CallParentFunction)
  (Components|Movement|StopMovementImmediately _charactermovement)
  (Variables|Default|SetJetpackState "NewEnumerator1")
  (Variables|/Script/Engine.MovementComponent|SetVelocity _charactermovement "0, 0, 0")
  (bind _asbp_character (Utilities|Casting|CastToBP_Character (Variables|Default|GetOwnerCharacter)))
  (Default|FXJetpack _asbp_character true))

(event EventUpdateAbility
  (params (DeltaTime :type Float%20%28single-precision%29))
  (|CallParentFunction DeltaTime)
  (switch Utilities|FlowControl|Switch|SwitchonELFJetPackState (Variables|Default|GetJetpackState)
    (:NewEnumerator1
      (bind _output_get (Variables|Default|SetCurrentJetpackTime (+ DeltaTime (Variables|Default|GetCurrentJetpackTime))))
      (if (>= _output_get (Variables|Default|GetMaxTime))
        (Class|LFAbilityComponent|DeactivateAbilitybyType (Actor|GetComponentbyClass (Variables|Default|GetOwnerCharacter) "/Script/LF.LFAbilityComponent") "Jetpack"))
      (Character|LaunchCharacter (Variables|Default|GetOwnerCharacter) (Math|Vector|MakeVector 0.0 0.0 (+ (/ (Variables|Default|GetMaxHeight) (Variables|Default|GetMaxTime)) 41.0)) false true))))

(event EventDeactivateAbility
  (|CallParentFunction)
  (Variables|Default|SetJetpackState "NewEnumerator2")
  (Character|LaunchCharacter (Variables|Default|GetOwnerCharacter) (Math|Vector|MakeVector 0.0 0.0 0.0) false true)
  (bind _asbp_character (Utilities|Casting|CastToBP_Character (Variables|Default|GetOwnerCharacter)))
  (Default|FXJetpack _asbp_character false))

(fn CanUseAbility
  (bind _returnvalue (|CallParentFunction))
  (return (Math|Boolean|ANDBoolean _returnvalue (Utilities|Enum|Equal(Enum) (Variables|Default|GetJetpackState) "NewEnumerator0") (Utilities|Enum|NotEqual(Enum) (Variables|/Script/LF.LFAbilityComponent|GetCurrentAbility (Variables|Default|GetOwnerAbilityComponent)) "Stomp"))))