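; Dash ability that launches the owning character forward in a straight, gravity-free burst.
; UseDash saves braking and gravity, zeroes both, switches the capsule to a profile ignoring dashing objects and sets a high forward velocity.
; Reaching the dash distance or hitting something deactivates it, restoring settings and zeroing velocity.
; Use requires an elapsed cooldown, no unlanded air dash and no active Stomp, otherwise failure FX plays.
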(event Custom|OnCapsuleHit
  (params (HitComponent :type Primitive%20Component%20Object%20Reference) (OtherActor :type Actor%20Object%20Reference) (OtherComp :type Primitive%20Component%20Object%20Reference) (NormalImpulse :type Vector) (Hit :type Hit%20Result%20Structure%20%28by%20ref%29))
  (if (Variables|Default|GetbIsDashing)
    (Class|LFAbility|DeactivateAbility)))

(event EventActivateAbility
  (|CallParentFunction)
  (CallFunction|UseDash))

(event EventBeginAbility
  (params (Character :type LF%20Character%20Object%20Reference) (AbilityComponent :type LF%20Ability%20Component%20Object%20Reference))
  (|CallParentFunction Character AbilityComponent)
  (bind _asbp_character (Utilities|Casting|CastToBP_Character (Variables|Default|GetOwnerCharacter)))
  (Collision|BindEventtoOnComponentHit (Variables|/Script/Engine.Character|GetCapsuleComponent _asbp_character) (delegate Custom|OnCapsuleHit))
  (Variables|Default|SetBrakingBeforeDash (Variables|/Script/Engine.CharacterMovementComponent|GetBrakingFrictionFactor (Variables|/Script/Engine.Character|GetCharacterMovement _asbp_character)))
  (Variables|Default|SetGravityBeforeDash (Variables|/Script/Engine.CharacterMovementComponent|GetGravityScale (Variables|/Script/Engine.Character|GetCharacterMovement _asbp_character))))

(event EventUpdateAbility
  (params (DeltaTime :type Float%20%28single-precision%29))
  (bind _ownercharacter (Variables|Default|GetOwnerCharacter))
  (|CallParentFunction DeltaTime)
  (if (Variables|Default|GetbIsDashing)
    (if (>= (Math|Vector|VectorLength (- (Variables|Default|GetPositionBeforeDash) (Transformation|GetActorLocation _ownercharacter))) (Variables|Default|GetDASHDISTANCE))
      (Class|LFAbility|DeactivateAbility))
    (else
      (Variables|Default|SetTimeFromLastDash (+ DeltaTime (Variables|Default|GetTimeFromLastDash)))
      (bind _asbp_character (Utilities|Casting|CastToBP_Character _ownercharacter))
      (if (not (AI|Components|NavMovement|IsFalling (Variables|/Script/Engine.Character|GetCharacterMovement _asbp_character)))
        (Variables|Default|SetbLastDashFromAir false)))))

(event EventDeactivateAbility
  (|CallParentFunction)
  (CallFunction|StopDash))

(fn UseDash
  (bind _ownercharacter (Variables|Default|GetOwnerCharacter))
  (bind _ownercharacter_2 (Variables|Default|GetOwnerCharacter))
  (bind _ownercharacter_3 (Variables|Default|GetOwnerCharacter))
  (bind _charactermovement (Variables|/Script/Engine.Character|GetCharacterMovement _ownercharacter_2))
  (bind _returnvalue (CallFunction|CanUseAbility))
  (if _returnvalue
    (Utilities|FlowControl|Sequence
      (:then_0
        (bind _asbp_character (Utilities|Casting|CastToBP_Character _ownercharacter_3))
        (Default|FXDash _asbp_character))
      (:then_1
        (Variables|Default|SetbIsDashing true)
        (Variables|Default|SetTimeFromLastDash 0.0)
        (Variables|Default|SetPositionBeforeDash (Transformation|GetActorLocation (Variables|Default|GetOwnerCharacter)))
        (Variables|Default|SetbLastDashFromAir (AI|Components|NavMovement|IsFalling _charactermovement))
        (Collision|SetCollisionProfileName (Variables|/Script/Engine.Character|GetCapsuleComponent (Variables|Default|GetOwnerCharacter)) "PawnIgnoreDashingObjects" true :!class /Script/Engine.PrimitiveComponent)
        (Variables|Default|SetBrakingBeforeDash (Variables|/Script/Engine.CharacterMovementComponent|GetBrakingFrictionFactor _charactermovement))
        (Variables|Default|SetGravityBeforeDash (Variables|/Script/Engine.CharacterMovementComponent|GetGravityScale _charactermovement))
        (Variables|/Script/Engine.CharacterMovementComponent|SetBrakingFrictionFactor _charactermovement 0.0)
        (Variables|/Script/Engine.CharacterMovementComponent|SetGravityScale _charactermovement 0.0)
        (Components|Movement|StopMovementImmediately (Variables|/Script/Engine.Character|GetCharacterMovement _ownercharacter))
        (Variables|/Script/Engine.MovementComponent|SetVelocity _charactermovement (* (Transformation|GetActorForwardVector _ownercharacter) 5e+03))))
    (else
      (bind _asbp_character_2 (Utilities|Casting|CastToBP_Character _ownercharacter_3))
      (Default|FXCantUseSkill _asbp_character_2 "Dash"))))

(fn StopDash
  (Variables|Default|SetbIsDashing false)
  (bind _asbp_character (Utilities|Casting|CastToBP_Character (Variables|Default|GetOwnerCharacter)))
  (Collision|SetCollisionProfileName (Variables|/Script/Engine.Character|GetCapsuleComponent _asbp_character) "Pawn" true :!class /Script/Engine.PrimitiveComponent)
  (Variables|/Script/Engine.CharacterMovementComponent|SetBrakingFrictionFactor (Variables|/Script/Engine.Character|GetCharacterMovement _asbp_character) (Variables|Default|GetBrakingBeforeDash))
  (Variables|/Script/Engine.CharacterMovementComponent|SetGravityScale (Variables|/Script/Engine.Character|GetCharacterMovement _asbp_character) (Variables|Default|GetGravityBeforeDash))
  (Variables|/Script/Engine.MovementComponent|SetVelocity (Variables|/Script/Engine.Character|GetCharacterMovement _asbp_character) "0, 0, 0"))

(fn GetCanDash
  (return (and (>= (Variables|Default|GetTimeFromLastDash) (Variables|Default|GetTIMEBETWEENDASHES)) (not (Variables|Default|GetbLastDashFromAir)))))

(fn CanUseAbility
  (bind _returnvalue (|CallParentFunction))
  (return (Math|Boolean|ANDBoolean _returnvalue (and (>= (Variables|Default|GetTimeFromLastDash) (Variables|Default|GetTIMEBETWEENDASHES)) (not (Variables|Default|GetbLastDashFromAir))) (Utilities|Enum|NotEqual(Enum) (Variables|/Script/LF.LFAbilityComponent|GetCurrentAbility (Variables|Default|GetOwnerAbilityComponent)) "Stomp"))))