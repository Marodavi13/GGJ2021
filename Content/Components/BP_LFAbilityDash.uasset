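; Dash ability component that launches the owning character forward in a straight, gravity-free burst.
; Activation zeroes braking friction and gravity and sets a high forward velocity, saving the old values to restore on stop.
; The dash ends after a set distance, on a capsule hit or on deactivation, halting all movement.
; Reuse requires a cooldown, and an air dash blocks further dashes until landing.
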(event Custom|OnCapsuleHit
  (params (HitComponent :type Primitive%20Component%20Object%20Reference) (OtherActor :type Actor%20Object%20Reference) (OtherComp :type Primitive%20Component%20Object%20Reference) (NormalImpulse :type Vector) (Hit :type Hit%20Result%20Structure%20%28by%20ref%29))
  (if (Variables|Default|GetbIsDashing)
    (Class|LFAbility|DeactivateAbility)))

(event EventActivateAbility
  (|CallParentFunction)
  (CallFunction|UseDash))

(event EventBeginAbility
  (params (Character :type LF%20Character%20Object%20Reference))
  (|CallParentFunction Character)
  (bind _asbp_character (Utilities|Casting|CastToBP_Character (Variables|Default|GetOwnerCharacter)))
  (Collision|BindEventtoOnComponentHit (Variables|/Script/Engine.Character|GetCapsuleComponent _asbp_character) (delegate Custom|OnCapsuleHit))
  (Variables|Default|SetBrakingBeforeDash (Variables|/Script/Engine.CharacterMovementComponent|GetBrakingFrictionFactor (Variables|/Script/Engine.Character|GetCharacterMovement _asbp_character)))
  (Variables|Default|SetGravityBeforeDash (Variables|/Script/Engine.CharacterMovementComponent|GetGravityScale (Variables|/Script/Engine.Character|GetCharacterMovement _asbp_character))))

(event EventUpdateAbility
  (params (DeltaTime :type Float%20%28single-precision%29))
  (bind _ownercharacter (Variables|Default|GetOwnerCharacter))
  (|CallParentFunction DeltaTime)
  (if (Variables|Default|GetbIsDashing)
    (if (>= (Math|Vector|VectorLength (- (Variables|Default|GetPositionBeforeDash) (Transformation|GetActorLocation _ownercharacter))) (Variables|Default|GetDASHDISTANCE))
      (Class|LFAbility|DeactivateAbility))
    (else
      (Variables|Default|SetTimeFromLastDash (+ DeltaTime (Variables|Default|GetTimeFromLastDash)))
      (bind _asbp_character (Utilities|Casting|CastToBP_Character _ownercharacter))
      (if (not (AI|Components|NavMovement|IsFalling (Variables|/Script/Engine.Character|GetCharacterMovement _asbp_character)))
        (Variables|Default|SetbLastDashFromAir false)))))

(event EventDeactivateAbility
  (|CallParentFunction)
  (CallFunction|StopDash))

(fn UseDash
  (bind _ownercharacter (Variables|Default|GetOwnerCharacter))
  (bind _returnvalue (CallFunction|CanUseAbility))
  (if _returnvalue
    (Variables|Default|SetbIsDashing true)
    (Variables|Default|SetTimeFromLastDash 0.0)
    (Variables|Default|SetPositionBeforeDash (Transformation|GetActorLocation _ownercharacter))
    (bind _asbp_character (Utilities|Casting|CastToBP_Character _ownercharacter))
    (Variables|/Script/LF.LFAnimationComponent|SetbIsDashing (Variables|/Script/LF.LFCharacter|GetAnimationComponent _asbp_character) true)
    (Variables|Default|SetbLastDashFromAir (AI|Components|NavMovement|IsFalling (Variables|/Script/Engine.Character|GetCharacterMovement _asbp_character)))
    (Variables|Default|SetBrakingBeforeDash (Variables|/Script/Engine.CharacterMovementComponent|GetBrakingFrictionFactor (Variables|/Script/Engine.Character|GetCharacterMovement _asbp_character)))
    (Variables|Default|SetGravityBeforeDash (Variables|/Script/Engine.CharacterMovementComponent|GetGravityScale (Variables|/Script/Engine.Character|GetCharacterMovement _asbp_character)))
    (Variables|/Script/Engine.CharacterMovementComponent|SetBrakingFrictionFactor (Variables|/Script/Engine.Character|GetCharacterMovement _asbp_character) 0.0)
    (Variables|/Script/Engine.CharacterMovementComponent|SetGravityScale (Variables|/Script/Engine.Character|GetCharacterMovement _asbp_character) 0.0)
    (Variables|/Script/Engine.MovementComponent|SetVelocity (Variables|/Script/Engine.Character|GetCharacterMovement _asbp_character) (* (Transformation|GetActorForwardVector _asbp_character) 5e+03))))

(fn StopDash
  (Variables|Default|SetbIsDashing false)
  (bind _asbp_character (Utilities|Casting|CastToBP_Character (Variables|Default|GetOwnerCharacter)))
  (Variables|/Script/LF.LFAnimationComponent|SetbIsDashing (Variables|/Script/LF.LFCharacter|GetAnimationComponent _asbp_character) false)
  (Variables|/Script/Engine.CharacterMovementComponent|SetBrakingFrictionFactor (Variables|/Script/Engine.Character|GetCharacterMovement _asbp_character) (Variables|Default|GetBrakingBeforeDash))
  (Variables|/Script/Engine.CharacterMovementComponent|SetGravityScale (Variables|/Script/Engine.Character|GetCharacterMovement _asbp_character) (Variables|Default|GetGravityBeforeDash))
  (Variables|/Script/Engine.MovementComponent|SetVelocity (Variables|/Script/Engine.Character|GetCharacterMovement _asbp_character) "0, 0, 0"))

(fn GetCanDash
  (return (and (>= (Variables|Default|GetTimeFromLastDash) (Variables|Default|GetTIMEBETWEENDASHES)) (not (Variables|Default|GetbLastDashFromAir)))))

(fn CanUseAbility
  (bind _returnvalue (|CallParentFunction))
  (return (and _returnvalue (and (>= (Variables|Default|GetTimeFromLastDash) (Variables|Default|GetTIMEBETWEENDASHES)) (not (Variables|Default|GetbLastDashFromAir))))))