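; BP_FallingComponent is an actor component that switches the owning BP_Character between the falling animation and none.
; It caches the owner on BeginPlay, then each tick checks whether the sprite's flipbook is idle, walk or falling.
; If so, and no ability is active, it uses CharacterMovement's falling state to set the animation through the character's AnimationComponent.
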(event EventBeginPlay
  (bind _asbp_character (Utilities|Casting|CastToBP_Character (Components|GetOwner)))
  (Variables|Default|SetOwnerCharacter _asbp_character))

(event EventTick
  (params (DeltaSeconds :type Float%20%28single-precision%29))
  (bind _ownercharacter (Variables|Default|GetOwnerCharacter))
  (bind _ownercharacter_2 (Variables|Default|GetOwnerCharacter))
  (bind _ownercharacter_3 (Variables|Default|GetOwnerCharacter))
  (bind _sprite (Variables|/Script/Paper2D.PaperCharacter|GetSprite _ownercharacter))
  (bind _abilitycomponent (Variables|/Game/2DSideScrollerCPP/Blueprints/BP_Character.BP_Character_C|GetAbilityComponent _ownercharacter_2))
  (bind _animationcomponent (Variables|/Script/LF.LFCharacter|GetAnimationComponent _ownercharacter_3))
  (bind _returnvalue (Class|LFAbilityComponent|GetCurrentAbilityType _abilitycomponent))
  (bind _returnvalue_2 (Class|PaperFlipbookComponent|GetFlipbook _sprite))
  (bind _returnvalue_3 (Utilities|Enum|Equal(Enum) _returnvalue "None"))
  (if (or (or (== _returnvalue_2 "/Game/Sprites/Character/IdleHD.IdleHD") (== _returnvalue_2 "/Game/Sprites/Character/Falling.Falling")) (== _returnvalue_2 "/Game/Sprites/Character/WalkHD.WalkHD"))
    (if (AI|Components|NavMovement|IsFalling (Variables|/Script/Engine.Character|GetCharacterMovement _ownercharacter_2))
      (if _returnvalue_3
        (Class|LFAnimationComponent|SetCurrentAnimation _animationcomponent "Falling"))
      (elif _returnvalue_3
        (Class|LFAnimationComponent|SetCurrentAnimation _animationcomponent "None")))))