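; BP_Stairs_2 is a stairs actor that tells BP_Character when it is at the stairs or at their top.
; Overlaps on Box and Box2 set and clear the character's IsInStairs and IsInStairsTop flags, respectively.
; Each tick, Box1 switches its Pawn collision response to Overlap while the player's IsInStairs is true, and to Block otherwise.
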(event Custom|OnBeginOverlap
  (params (OverlappedComponent :type Primitive%20Component%20Object%20Reference) (OtherActor :type Actor%20Object%20Reference) (OtherComp :type Primitive%20Component%20Object%20Reference) (OtherBodyIndex :type Integer) (bFromSweep :type Boolean) (SweepResult :type Hit%20Result%20Structure%20%28by%20ref%29))
  (bind _asbp_character (Utilities|Casting|CastToBP_Character OtherActor))
  (Variables|/Game/2DSideScrollerCPP/Blueprints/BP_Character.BP_Character_C|SetbIsInStairs _asbp_character true))

(event Custom|OnEndOverlap
  (params (OverlappedComponent :type Primitive%20Component%20Object%20Reference) (OtherActor :type Actor%20Object%20Reference) (OtherComp :type Primitive%20Component%20Object%20Reference) (OtherBodyIndex :type Integer))
  (bind _asbp_character (Utilities|Casting|CastToBP_Character OtherActor))
  (Variables|/Game/2DSideScrollerCPP/Blueprints/BP_Character.BP_Character_C|SetbIsInStairs _asbp_character false))

(event Custom|OnBeginOverlapTop
  (params (OverlappedComponent :type Primitive%20Component%20Object%20Reference) (OtherActor :type Actor%20Object%20Reference) (OtherComp :type Primitive%20Component%20Object%20Reference) (OtherBodyIndex :type Integer) (bFromSweep :type Boolean) (SweepResult :type Hit%20Result%20Structure%20%28by%20ref%29))
  (bind _asbp_character (Utilities|Casting|CastToBP_Character OtherActor))
  (Variables|/Game/2DSideScrollerCPP/Blueprints/BP_Character.BP_Character_C|SetbIsInStairsTop _asbp_character true))

(event Custom|OnEndOverlapTop
  (params (OverlappedComponent :type Primitive%20Component%20Object%20Reference) (OtherActor :type Actor%20Object%20Reference) (OtherComp :type Primitive%20Component%20Object%20Reference) (OtherBodyIndex :type Integer))
  (bind _asbp_character (Utilities|Casting|CastToBP_Character OtherActor))
  (Variables|/Game/2DSideScrollerCPP/Blueprints/BP_Character.BP_Character_C|SetbIsInStairsTop _asbp_character false))

(event EventBeginPlay
  (bind _box (Variables|Default|GetBox))
  (bind _box2 (Variables|Default|GetBox2))
  (Collision|BindEventtoOnComponentBeginOverlap _box (delegate Custom|OnBeginOverlap))
  (Collision|BindEventtoOnComponentEndOverlap _box (delegate Custom|OnEndOverlap))
  (Collision|BindEventtoOnComponentBeginOverlap _box2 (delegate Custom|OnBeginOverlapTop))
  (Collision|BindEventtoOnComponentEndOverlap _box2 (delegate Custom|OnEndOverlapTop)))

(event EventTick
  (params (DeltaSeconds :type Float%20%28single-precision%29))
  (bind _box1 (Variables|Default|GetBox1))
  (bind _asbp_character (Utilities|Casting|CastToBP_Character (Pawn|GetControlledPawn (Game|GetPlayerController 0))))
  (if (Variables|/Game/2DSideScrollerCPP/Blueprints/BP_Character.BP_Character_C|GetbIsInStairs _asbp_character)
    (Collision|SetCollisionResponsetoChannel _box1 "ECC_Pawn" "ECR_Overlap")
    (else
      (Collision|SetCollisionResponsetoChannel _box1 "ECC_Pawn" "ECR_Block"))))

(fn ConstructionScript)