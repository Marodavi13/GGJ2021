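; Altar actor that takes its assigned ability away from an overlapping character who has it, and can activate only once.
; Activation disables the ability, notifies the character, plays a sound and runs a timeline moving the orb sprite to its altar position.
; A second timeline then fades in eye and glow sprites alongside an ability-specific particle burst.
; On/off sprite sets come from default content per ability, also applied in the construction script.
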(event OnComponentBeginOverlap(Overlap)
  (params (OverlappedComponent :type Primitive%20Component%20Object%20Reference) (OtherActor :type Actor%20Object%20Reference) (OtherComp :type Primitive%20Component%20Object%20Reference) (OtherBodyIndex :type Integer) (bFromSweep :type Boolean) (SweepResult :type Hit%20Result%20Structure%20%28by%20ref%29))
  ;[1 1 1] Character Interaction
  (bind _asbp_character (Utilities|Casting|CastToBP_Character OtherActor))
  (Variables|Default|SetCharacter _asbp_character)
  (if (and (Class|LFAbilityComponent|IsAbilityAllowed (Variables|/Game/2DSideScrollerCPP/Blueprints/BP_Character.BP_Character_C|GetAbilityComponent _asbp_character) (Variables|Default|GetAltarAbility)) (Variables|Default|GetbIsAltarActivable))
    (CallFunction|ActivateAltar)))

(event Custom|ActivateAltar
  ;[1 1 1] Activate Altar
  (Variables|Default|SetbIsAltarActivable false)
  (Default|OnOrbPicked (Variables|Default|GetCharacter) (Variables|Default|GetAltarAbility))
  (Class|LFAbilityComponent|AllowAbility (Variables|/Game/2DSideScrollerCPP/Blueprints/BP_Character.BP_Character_C|GetAbilityComponent (Variables|Default|GetCharacter)) (Variables|Default|GetAltarAbility) false)
  (Variables|Default|SetOrbEnd (Transformation|GetWorldLocation (Variables|Default|GetOrbSprite)))
  (bind _output_get (Variables|Default|SetOrbStart (|CalculateOrbStart)))
  (Transformation|SetWorldLocation (Variables|Default|GetOrbSprite) _output_get false false)
  (CallFunction|UpdateAltarVisuals true)
  (Audio|PlaySound2D "/Game/SFX/objectives/Cue_Objective.Cue_Objective" 1.0 1.0 0.0 0 0)
  (bind _newtrack_0 (Timeline|Move%20orb%20to%20altar PlayFromStart)
    (:Update
      (Transformation|SetWorldLocation (Variables|Default|GetOrbSprite) (Math|Vector|Lerp(Vector) (Variables|Default|GetOrbStart) (Variables|Default|GetOrbEnd) _newtrack_0) false false))
    (:Finished
      (CallFunction|AnimateGlow)
      ;[1 1 1] vfx
      (Effects|SpawnEmitteratLocation (Utilities|Select :Index (Variables|Default|GetAltarAbility) :None "/Game/VFX/Par_ToonKaboom_01.Par_ToonKaboom_01" :Jump "/Game/VFX/Par_ToonKaboom_01.Par_ToonKaboom_01" :Jetpack "/Game/VFX/Par_ToonKaboom_01_verde.Par_ToonKaboom_01_verde" :Dash "/Game/VFX/Par_ToonKaboom_01_rojo.Par_ToonKaboom_01_rojo" :Stomp "/Game/VFX/Par_ToonKaboom_01.Par_ToonKaboom_01" :Count "/Game/VFX/Par_ToonKaboom_01.Par_ToonKaboom_01") (Transformation|GetWorldLocation (Variables|Default|GetScene))))))

(event Custom|UpdateAltarVisuals
  (params (bHideSprites :type Boolean))
  ;[1 1 1] Update Altar visuals based on the activated bool
  (if bHideSprites
    (Sprite|SetSpriteColor (Variables|Default|GetEyesSprite) (Utilities|Struct|MakeLinearColor 1.0 1.0 1.0 0.0))
    (Sprite|SetSpriteColor (Variables|Default|GetGlowSprite) (Utilities|Struct|MakeLinearColor 1.0 1.0 1.0 0.0))
    (else
      (Sprite|SetSpriteColor (Variables|Default|GetEyesSprite) (Utilities|Struct|MakeLinearColor 1.0 1.0 1.0 1.0))
      (Sprite|SetSpriteColor (Variables|Default|GetGlowSprite) (Utilities|Struct|MakeLinearColor 1.0 1.0 1.0 1.0))))
  (if (Variables|Default|GetbIsAltarActivable)
    (bind _returnvalue (Class|LFDefaultContent|GetOffAltarSprites (Class|LFLibrary|GetLFDefaultContent) (Variables|Default|GetAltarAbility)))
    (CallFunction|SetSprites _returnvalue)
    (else
      (bind _returnvalue_2 (Class|LFDefaultContent|GetonAltarSprites (Class|LFLibrary|GetLFDefaultContent) (Variables|Default|GetAltarAbility)))
      (CallFunction|SetSprites _returnvalue_2))))

(event Custom|SetSprites
  (params (Sprites :type Array%20of%20Paper%20Sprite%20Object%20References))
  (Rendering|Components|Sprite|SetSprite (Variables|Default|GetAltarSprite) (Utilities|Array|Get(acopy) Sprites))
  (Rendering|Components|Sprite|SetSprite (Variables|Default|GetEyesSprite) (Utilities|Array|Get(acopy) Sprites 1))
  (Rendering|Components|Sprite|SetSprite (Variables|Default|GetGlowSprite) (Utilities|Array|Get(acopy) Sprites 2))
  (Rendering|Components|Sprite|SetSprite (Variables|Default|GetOrbSprite) (Utilities|Array|Get(acopy) Sprites 3)))

(event Custom|AnimateGlow
  (bind _newtrack_0 (Timeline|Glow PlayFromStart)
    (:Update
      (Sprite|SetSpriteColor (Variables|Default|GetGlowSprite) (Utilities|Struct|MakeLinearColor 1.0 1.0 1.0 _newtrack_0))
      (Sprite|SetSpriteColor (Variables|Default|GetEyesSprite) (Utilities|Struct|MakeLinearColor 1.0 1.0 1.0 _newtrack_0))
      (Development|PrintString (Utilities|String|ToString(Float) _newtrack_0)))))

(event EventBeginPlay)

(event Collision|EventActorBeginOverlap
  (params (OtherActor :type Actor%20Object%20Reference)))

(event EventTick
  (params (DeltaSeconds :type Float%20%28single-precision%29)))

(fn ConstructionScript
  (CallFunction|UpdateAltarVisuals false))