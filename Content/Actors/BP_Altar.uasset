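; One-shot altar actor that takes its assigned ability away from an overlapping BP_Character that has it allowed.
; Activation notifies the character, disallows the ability and runs a timeline moving the orb from CalculateOrbStart's result to its resting spot.
; CalculateOrbStart's above-character position math is left unused.
; The construction script and UpdateAltarVisuals duplicate state visuals: dimmed ability color with hidden orb while activatable, full color with visible orb afterwards.
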(event OnComponentBeginOverlap(Overlap)
  (params (OverlappedComponent :type Primitive%20Component%20Object%20Reference) (OtherActor :type Actor%20Object%20Reference) (OtherComp :type Primitive%20Component%20Object%20Reference) (OtherBodyIndex :type Integer) (bFromSweep :type Boolean) (SweepResult :type Hit%20Result%20Structure%20%28by%20ref%29))
  ;[1 1 1] Character Interaction
  (bind _asbp_character (Utilities|Casting|CastToBP_Character OtherActor))
  (Variables|Default|SetCharacter _asbp_character)
  (bind _returnvalue (Class|LFAbilityComponent|IsAbilityAllowed (Variables|/Game/2DSideScrollerCPP/Blueprints/BP_Character.BP_Character_C|GetAbilityComponent _asbp_character) (Variables|Default|GetAltarAbility)))
  (if (and _returnvalue (Variables|Default|GetbIsAltarActivable))
    (CallFunction|ActivateAltar)))

(event Custom|ActivateAltar
  ;[1 1 1] Activate Altar
  (Variables|Default|SetbIsAltarActivable false)
  (Default|OnOrbPicked (Variables|Default|GetCharacter) (Variables|Default|GetAltarAbility))
  (Class|LFAbilityComponent|AllowAbility (Variables|/Game/2DSideScrollerCPP/Blueprints/BP_Character.BP_Character_C|GetAbilityComponent (Variables|Default|GetCharacter)) (Variables|Default|GetAltarAbility) false)
  (Variables|Default|SetOrbEnd (Transformation|GetWorldLocation (Variables|Default|GetOrb)))
  (bind _output_get (Variables|Default|SetOrbStart (|CalculateOrbStart)))
  (Transformation|SetWorldLocation (Variables|Default|GetOrb) _output_get false false)
  (CallFunction|UpdateAltarVisuals)
  (bind _newtrack_0 (Timeline|Move%20orb%20to%20altar PlayFromStart)
    (:Update
      (Transformation|SetWorldLocation (Variables|Default|GetOrb) (Math|Vector|Lerp(Vector) (Variables|Default|GetOrbStart) (Variables|Default|GetOrbEnd) _newtrack_0) false false))))

(event Custom|UpdateAltarVisuals
  (bind _returnvalue (Class|LFLibrary|GetLFDefaultContent))
  (bind _returnvalue_2 (Class|LFLibrary|GetLFDefaultContent))
  (bind _altarability (Variables|Default|GetAltarAbility))
  (bind _altarability_2 (Variables|Default|GetAltarAbility))
  (bind _returnvalue_3 (Class|LFDefaultContent|GetAbilityColor _returnvalue _altarability))
  (bind _returnvalue_4 (Class|LFDefaultContent|GetAbilityColor _returnvalue_2 _altarability_2))
  (bind _returnvalue_5 (* _returnvalue_4 0.1))
  (bind (_r _g _b) (Math|Color|BreakColor _returnvalue_3))
  (bind (_r_2 _g_2 _b_2) (Math|Color|BreakColor _returnvalue_5))
  ;[1 1 1] Update Altar visuals based on the activated bool
  (if (Variables|Default|GetbIsAltarActivable)
    (Sprite|SetSpriteColor (Variables|Default|GetAltarSprite) (Utilities|Struct|MakeLinearColor _r_2 _g_2 _b_2 1.0))
    (Rendering|SetVisibility (Variables|Default|GetOrb) false false)
    (else
      (Sprite|SetSpriteColor (Variables|Default|GetAltarSprite) (Utilities|Struct|MakeLinearColor _r _g _b 1.0))
      (Sprite|SetSpriteColor (Variables|Default|GetOrb) (Utilities|Struct|MakeLinearColor _r _g _b 1.0))
      (Rendering|SetVisibility (Variables|Default|GetOrb) true false))))

(event EventBeginPlay)

(event Collision|EventActorBeginOverlap
  (params (OtherActor :type Actor%20Object%20Reference)))

(event EventTick
  (params (DeltaSeconds :type Float%20%28single-precision%29)))

(fn ConstructionScript
  (bind _returnvalue (Class|LFLibrary|GetLFDefaultContent))
  (bind _returnvalue_2 (Class|LFLibrary|GetLFDefaultContent))
  (bind _altarability (Variables|Default|GetAltarAbility))
  (bind _altarability_2 (Variables|Default|GetAltarAbility))
  (bind _returnvalue_3 (Class|LFDefaultContent|GetAbilityColor _returnvalue _altarability))
  (bind _returnvalue_4 (Class|LFDefaultContent|GetAbilityColor _returnvalue_2 _altarability_2))
  (bind _returnvalue_5 (* _returnvalue_4 0.1))
  (bind (_r _g _b) (Math|Color|BreakColor _returnvalue_3))
  (bind (_r_2 _g_2 _b_2) (Math|Color|BreakColor _returnvalue_5))
  (if (Variables|Default|GetbIsAltarActivable)
    (Sprite|SetSpriteColor (Variables|Default|GetAltarSprite) (Utilities|Struct|MakeLinearColor _r_2 _g_2 _b_2 1.0))
    (Rendering|SetVisibility (Variables|Default|GetOrb) false false)
    (else
      (Sprite|SetSpriteColor (Variables|Default|GetAltarSprite) (Utilities|Struct|MakeLinearColor _r _g _b 1.0))
      (Sprite|SetSpriteColor (Variables|Default|GetOrb) (Utilities|Struct|MakeLinearColor _r _g _b 1.0))
      (Rendering|SetVisibility (Variables|Default|GetOrb) true false))))