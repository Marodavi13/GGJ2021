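; BP_Ledge is a one-way platform map module built on a Paper2D sprite.
; It caches player 0's BP_Character on BeginPlay, then each Tick compares the bottom of that character's capsule to a fixed height offset above the sprite.
; The sprite blocks the Pawn collision channel when the character is at or above that height and ignores it otherwise, switching for all pawns based on that one character.
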(event Custom|IgnorePlayer
  (Collision|SetCollisionResponsetoChannel (Variables|Default|GetPaperSprite) "ECC_Pawn" "ECR_Ignore"))

(event Custom|BlockPlayer
  (Collision|SetCollisionResponsetoChannel (Variables|Default|GetPaperSprite) "ECC_Pawn" "ECR_Block"))

(event EventBeginPlay
  (|CallParentFunction)
  (bind _asbp_character (Utilities|Casting|CastToBP_Character (Pawn|GetControlledPawn (Game|GetPlayerController 0))))
  (Variables|Default|SetCharacter _asbp_character))

(event Collision|EventActorBeginOverlap
  (params (OtherActor :type Actor%20Object%20Reference))
  (|CallParentFunction OtherActor) ; This node is disabled and will not be called.\nDrag off pins to build functionality.
)

(event EventTick
  (params (DeltaSeconds :type Float%20%28single-precision%29))
  (|CallParentFunction DeltaSeconds)
  (bind _character (Variables|Default|GetCharacter)
    (:then
      (if (>= (- (- (.z (Transformation|GetActorLocation _character)) (Variables|/Script/Engine.CapsuleComponent|GetCapsuleHalfHeight (Variables|/Script/Engine.Character|GetCapsuleComponent _character))) (+ (.z (Transformation|GetWorldLocation (Variables|Default|GetPaperSprite))) 1.2e+02)) 0.0)
        (CallFunction|BlockPlayer)
        (else
          (CallFunction|IgnorePlayer))))
    (:else)))

(fn ConstructionScript
  (|CallParentFunction))