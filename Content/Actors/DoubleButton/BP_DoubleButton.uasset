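; BP_DoubleButton is a two-part actor that toggles between a raised and lowered position.
; On BeginPlay, LowPartIsGate and HighPartIsGate decide whether each part keeps its gate or regular child actor, destroying the other.
; A BP_Character using the Jetpack ability that overlaps LowBox shifts the whole actor up.
; A successful stomp through BP_StompBreakableComponent shifts it back down, with HighPartActive tracking state and a sound on each switch.
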(event OnSuccessfulStomp(BP_StompBreakableComponent)
  (if (Variables|Default|GetbHighPartActive)
    (Transformation|SetActorLocation (+ (Transformation|GetActorLocation) "0,0.000000,-300.000000") false false)
    (Variables|Default|SetbHighPartActive false)
    (Audio|PlaySound2D "/Game/SFX/jetpack/Cue_HeadHit.Cue_HeadHit" 1.0 1.0 0.0 0 0)))

(event Custom|OnOverlapLow
  (params (OverlappedComponent :type Primitive%20Component%20Object%20Reference) (OtherActor :type Actor%20Object%20Reference) (OtherComp :type Primitive%20Component%20Object%20Reference) (OtherBodyIndex :type Integer) (bFromSweep :type Boolean) (SweepResult :type Hit%20Result%20Structure%20%28by%20ref%29))
  (if (not (Variables|Default|GetbHighPartActive))
    (bind _asbp_character (Utilities|Casting|CastToBP_Character OtherActor))
    (if (Utilities|Enum|Equal(Enum) (Class|LFAbilityComponent|GetCurrentAbilityType (Variables|/Game/2DSideScrollerCPP/Blueprints/BP_Character.BP_Character_C|GetAbilityComponent _asbp_character)) "Jetpack")
      (Transformation|SetActorLocation (+ (Transformation|GetActorLocation) "0,0.000000,300.000000") false false)
      (Variables|Default|SetbHighPartActive true)
      (Audio|PlaySound2D "/Game/SFX/jetpack/Cue_HeadHit.Cue_HeadHit" 1.0 1.0 0.0 0 0))))

(event EventBeginPlay
  (Collision|BindEventtoOnComponentBeginOverlap (Variables|Default|GetLowBox) (delegate Custom|OnOverlapLow))
  (if (Variables|Default|GetbHighPartIsGate)
    (Components|DestroyComponent (Variables|Default|GetHighChildActor))
    (else
      (Components|DestroyComponent (Variables|Default|GetHighChildActorGate))))
  (if (Variables|Default|GetbLowPartIsGate)
    (Components|DestroyComponent (Variables|Default|GetLowChildActor))
    (else
      (Components|DestroyComponent (Variables|Default|GetLowChildActorGate)))))

(event Collision|EventActorBeginOverlap
  (params (OtherActor :type Actor%20Object%20Reference)))

(event EventTick
  (params (DeltaSeconds :type Float%20%28single-precision%29)))

(fn ConstructionScript)