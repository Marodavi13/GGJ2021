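; BP_Controller is a controller Blueprint that implements hold-to-restart for the level.
; On BeginPlay it caches the HUD object from BP_HUD and notifies it when the Restart input is pressed, passing the required hold time, or released.
; While the input is held, Tick accumulates time and calls RestartLevel on BP_GameModeBase once the threshold is exceeded.
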(event EventBeginPlay
  (bind _asbp_hud (Utilities|Casting|CastToBP_HUD (HUD|GetHUD)))
  (Variables|Default|SetHUD (Variables|/Game/UI/HUD/BP_HUD.BP_HUD_C|GetHUD _asbp_hud)))

(event EventTick
  (params (DeltaSeconds :type Float%20%28single-precision%29))
  (if (Variables|Default|GetbRestart)
    (bind _output_get (Variables|Default|SetCurrentTime (+ DeltaSeconds (Variables|Default|GetCurrentTime))))
    (if (> _output_get (Variables|Default|GetTimeToRestart))
      (bind _asbp_game_mode_base (Utilities|Casting|CastToBP_GameModeBase (Game|GetGameMode)))
      (Default|RestartLevel _asbp_game_mode_base))))

(event Input|ActionEvents|InputActionRestart
  (params (Key :type Key%20Structure :default "None"))
  (:Pressed
    (Variables|Default|SetCurrentTime 0.0)
    (Variables|Default|SetbRestart true)
    (Default|Restart (Variables|Default|GetHUD) (Variables|Default|GetTimeToRestart)))
  (:Released
    (Variables|Default|SetbRestart false)
    (Default|RestartReleased (Variables|Default|GetHUD))))

(fn ConstructionScript)